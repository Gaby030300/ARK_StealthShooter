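; BP_Enemy is an enemy Blueprint that displays its health and AI status as colored text.
; HealthComponent events update the health text, tint it by threshold through GetColorFromHealth, and hide it on death.
; SetEnemyStatus switches the status label and color between Patrol, Investigating and Combat.
; Point damage is forwarded to AI perception through ReportDamageEvent, with that handler bound inside the health-changed event rather than at BeginPlay.
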(event `self.ReceiveBeginPlay`
  (bind _healthtext (`self.HealthText`))
  ;[0.7024 0.5649 1] Text Health Info
  (`TextRenderComponent.K2_SetText` _healthtext (`KismetTextLibrary.Conv_DoubleToText` (`STS_HealthComponent.CurrentHealth` (`self.HealthComponent`)) "HalfToEven"))
  (`TextRenderComponent.SetTextRenderColor` _healthtext (`self.HealthyColor`)))

(event `self.HealthComponent.OnHealthChanged`
  (params (HealthComp :type "STS_HealthComponent Object Reference") (Health :type "Float (single-precision)") (HealthDelta :type "Float (single-precision)") (DamageType :type "DamageType Object Reference") (InstigatedBy :type "Controller Object Reference") (DamageCauser :type "Actor Object Reference"))
  (bind _healthtext (`self.HealthText`))
  ;[0.7024 0.5649 1] Text Health Info
  (`TextRenderComponent.K2_SetText` _healthtext (`KismetTextLibrary.Conv_DoubleToText` Health "HalfToEven"))
  (bind _numbercolor (`self.GetColorFromHealth` Health))
  (`TextRenderComponent.SetTextRenderColor` _healthtext _numbercolor)
  (add `Actor.OnTakePointDamage` (delegate `OnReportPointDamage`)))

(event `OnReportPointDamage`
  (params (DamagedActor :type "Actor Object Reference") (Damage :type "Float (double-precision)") (InstigatedBy :type "Controller Object Reference") (HitLocation :type "Vector Structure") (FHitComponent :type "PrimitiveComponent Object Reference") (BoneName :type Name) (ShotFromDirection :type "Vector Structure") (DamageType :type "DamageType Object Reference") (DamageCauser :type "Actor Object Reference"))
  ;[0.7024 0.5649 1] Text Health Info
  (`AISense_Damage.ReportDamageEvent` DamagedActor DamageCauser Damage HitLocation))

(event `self.HealthComponent.OnDeath`
  (params (HealthComp :type "STS_HealthComponent Object Reference") (InstigatedBy :type "Controller Object Reference") (Killer :type "Actor Object Reference"))
  ;[0.7024 0.5649 1] Text Health Info
  (`SceneComponent.SetVisibility` (`self.HealthText`) false false))

(event `self.BP_SetEnemyStatus`
  (params (NewEnemyStatus :type "ESTS_EnemyStatus Enum" :default "EnemyStatus_Patrol"))
  (`TextRenderComponent.K2_SetText` (`self.StatusText`) (select `ESTS_EnemyStatus` NewEnemyStatus :`EnemyStatus_Patrol` "Patrol" :`EnemyStatus_Investigating` "Investigating" :`EnemyStatus_Combat` "Combat"))
  (`TextRenderComponent.SetTextRenderColor` (`self.StatusText`) (select `ESTS_EnemyStatus` NewEnemyStatus :`EnemyStatus_Investigating` (`self.InvestigatingColor`) :`EnemyStatus_Combat` (`self.CombatColor`))))

(fn `GetColorFromHealth`
  (params (Health_Enemy :type "Float (double-precision)"))
  (returns (NumberColor :type "Color Structure"))
  (if (> Health_Enemy 80.0)
    (return (`self.HealthyColor`))
    (elif (> Health_Enemy 30.0)
      (return (`self.HurtColor`))
      (else
        (return (`self.CriticalColor`))))))

(fn `UserConstructionScript`)